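; BP_2ndDonKeyPickup is a key pickup actor that adds a key to the player's slots.
; On PickupCursorEvent it casts player character 0 to BP_Player and sets the first of three key slot variables that equals 0 to 1.
; It destroys itself once a slot is filled, and stays in the world if none is free.
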(event `PickupCursorEvent`
  ;[1 1 1] Key Pickup
  (bind _asbp_player (cast `/Game/Blueprints/BP_Player` (`GameplayStatics.GetPlayerCharacter` 0)))
  (if (== (`/Game/Blueprints/BP_Player.Slot1Key` _asbp_player) 0)
    (set `/Game/Blueprints/BP_Player.Slot1Key` 1 _asbp_player)
    (`self.K2_DestroyActor` :!label _label)
    (elif (== (`/Game/Blueprints/BP_Player.Slot2Key` _asbp_player) 0)
      (set `/Game/Blueprints/BP_Player.Slot2Key` 1 _asbp_player)
      (goto _label)
      (elif (== (`/Game/Blueprints/BP_Player.Slot3Key` _asbp_player) 0)
        (set `/Game/Blueprints/BP_Player.Slot3Key` 1 _asbp_player)
        (goto _label)))))

(fn `UserConstructionScript`)