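; Player character Blueprint that handles movement, mouse look, the HUD, a pause menu and close-range interaction.
; Axis inputs move relative to control yaw, and BeginPlay adds the HUD widget.
; Escape and M share one FlipFlop that toggles the pause menu, game pause and mouse cursor.
; Two separate left-click handlers each run a short, debug-drawn trace along the capsule's forward vector, opening a Door or triggering BP_1stDonKeyPickup's pickup event.
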(event `InputAxis|MoveForward`
  (params (AxisValue :type "Float (single-precision)"))
  ;[1 1 1] Player controller
  (`self.AddMovementInput` (`KismetMathLibrary.GetForwardVector` (`KismetMathLibrary.MakeRotator` 0.0 0.0 (.yaw (`self.GetControlRotation`)))) AxisValue))

(event `InputAxis|MoveRight`
  (params (AxisValue :type "Float (single-precision)"))
  ;[1 1 1] Player controller
  (`self.AddMovementInput` (`KismetMathLibrary.GetRightVector` (`KismetMathLibrary.MakeRotator` 0.0 0.0 (.yaw (`self.GetControlRotation`)))) AxisValue))

(event `InputAxis|Turn`
  (params (AxisValue :type "Float (single-precision)"))
  ;[1 1 1] Player controller
  (`self.AddControllerYawInput` AxisValue))

(event `InputAxis|LookUp`
  (params (AxisValue :type "Float (single-precision)"))
  ;[1 1 1] Player controller
  (`self.AddControllerPitchInput` AxisValue))

(event `Key|Escape`
  (params (Key :type "Key Structure"))
  (bind _returnvalue (`GameplayStatics.GetPlayerController` 0))
  ;[1 1 1] Pause menu
  (:`Pressed`
    (`/Engine/EditorBlueprintResources/StandardMacros.FlipFlop` :!label _label
      (:`A`
        (bind _returnvalue_2 (`|CreateWidget` "/Game/Widgets/WB_PauseMenu.WB_PauseMenu_C"))
        (`UserWidget.AddToViewport` _returnvalue_2 0)
        (`GameplayStatics.SetGamePaused` true)
        (set `PlayerController.bShowMouseCursor` true _returnvalue))
      (:`B`
        (`Widget.RemoveFromParent` _returnvalue_2)
        (`GameplayStatics.SetGamePaused` false)
        (set `PlayerController.bShowMouseCursor` false _returnvalue)))))

(event `Key|M` :paused true
  (params (Key :type "Key Structure"))
  ;[1 1 1] Pause menu
  (:`Pressed`
    (goto _label)))

(event `self.ReceiveBeginPlay`
  ;[1 1 1] HUD
  (bind _returnvalue (`|CreateWidget` "/Game/Blueprints/W_HUD.W_HUD_C"))
  (`UserWidget.AddToViewport` _returnvalue 0))

(event `Key|LeftMouseButton`
  (params (Key :type "Key Structure"))
  (bind _capsulecomponent (`self.CapsuleComponent`))
  (bind _returnvalue (`SceneComponent.K2_GetComponentLocation` _capsulecomponent))
  (:`Pressed`
    (bind _outhit (`KismetSystemLibrary.LineTraceSingle` :`Start` _returnvalue :`End` (+ _returnvalue (* (`SceneComponent.GetForwardVector` _capsulecomponent) 150.0)) :`TraceChannel` "TraceTypeQuery1" :`DrawDebugType` "ForDuration"))
    (bind _asdoor (cast `/Game/Blueprints/Door` (`.HitActor` (`GameplayStatics.BreakHitResult` _outhit))))
    (`/Game/Blueprints/Door.OpenDoor` _asdoor)))

(event `Key|LeftMouseButton`
  (params (Key :type "Key Structure"))
  (bind _capsulecomponent (`self.CapsuleComponent`))
  (bind _returnvalue (`SceneComponent.K2_GetComponentLocation` _capsulecomponent))
  (:`Pressed`
    (bind _outhit (`KismetSystemLibrary.LineTraceSingle` :`Start` _returnvalue :`End` (+ _returnvalue (* (`SceneComponent.GetForwardVector` _capsulecomponent) 150.0)) :`TraceChannel` "TraceTypeQuery1" :`DrawDebugType` "ForDuration"))
    (bind _asbp_1st_don_key_pickup (cast `/Game/Blueprints/BP_1stDonKeyPickup` (`.HitActor` (`GameplayStatics.BreakHitResult` _outhit))))
    (`/Game/Blueprints/BP_1stDonKeyPickup.PickupCursorEvent` _asbp_1st_don_key_pickup)))

(fn `UserConstructionScript`)