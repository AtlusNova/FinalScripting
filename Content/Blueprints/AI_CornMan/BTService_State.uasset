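; Behavior tree service for BP_CornMan AI that drives a state enum on the blackboard from AI perception.
; Each tick it loops through the pawn's perceived actors and, on a valid one, switches StateKey to the second enum value.
; After a three-second Delay inside the loop, it reverts to the first value and breaks; invalid entries also set the first value.
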(event `self.ReceiveTickAI`
  (params (OwnerController :type "AIController Object Reference") (ControlledPawn :type "Pawn Object Reference") (DeltaSeconds :type "Float (single-precision)"))
  (bind _asbp_corn_man (cast `/Game/Blueprints/BP_CornMan` ControlledPawn))
  (for _array_element (`AIPerceptionComponent.GetPerceivedActors` (`/Game/Blueprints/BP_CornMan.AIPerception` _asbp_corn_man) null)
    (`/Engine/EditorBlueprintResources/StandardMacros.IsValid` _array_element
      (:`Is Valid`
        (bind _output_get (set `self.State` "NewEnumerator1"))
        (`BTFunctionLibrary.SetBlackboardValueAsEnum` (`self.StateKey`) _output_get)
        (`KismetSystemLibrary.Delay` 3.0)
        (bind _output_get_2 (set `self.State` "NewEnumerator0"))
        (`BTFunctionLibrary.SetBlackboardValueAsEnum` (`self.StateKey`) _output_get_2)
        (break))
      (:`Is Not Valid`
        (bind _output_get_3 (set `self.State` "NewEnumerator0"))
        (`BTFunctionLibrary.SetBlackboardValueAsEnum` (`self.StateKey`) _output_get_3)))))